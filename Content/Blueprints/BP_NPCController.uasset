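; BP_NPCController is an NPC controller that sends its pawn toward a spot in front of the player.
; On BeginPlay it waits briefly, then calls SimpleMoveToLocation on itself with a goal offset along the player pawn's forward vector, computed only once.
; An unconnected AIMoveTo branch with debug prints targets the player pawn instead and never runs.
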(event `self.ReceiveBeginPlay`
  (bind _returnvalue (`GameplayStatics.GetPlayerPawn` 0))
  (`KismetSystemLibrary.Delay` 2.0)
  (`AIBlueprintHelperLibrary.SimpleMoveToLocation` self (+ (`self.K2_GetActorLocation` _returnvalue) (* (`self.GetActorForwardVector` _returnvalue) 500.0))))

(fn `UserConstructionScript`)